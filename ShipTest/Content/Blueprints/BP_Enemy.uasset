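; BP_Enemy is an enemy pawn that chases the player on sight and shoots at them.
; On PawnSensing detection it uses AIMoveTo, turns toward the player and spawns BP_BulletEnemy at PointerEnemy through a delay-reset DoOnce.
; Overlaps with "Bullet"-tagged actors reduce health and can increment BP_Main's kill count.
; Tick updates the WB_EnemyHealth bar, regenerates health after a post-hit delay and separately destroys the enemy at near-zero health.
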(event OnSeePawn(PawnSensing)
  (params (Pawn :type Pawn%20Object%20Reference))
  ;[1 1 1] IA
  (CallFunction|FollowPlayer))

(event OnComponentBeginOverlap(Sphere1)
  (params (OverlappedComponent :type Primitive%20Component%20Object%20Reference) (OtherActor :type Actor%20Object%20Reference) (OtherComp :type Primitive%20Component%20Object%20Reference) (OtherBodyIndex :type Integer) (bFromSweep :type Boolean) (SweepResult :type Hit%20Result%20Structure%20%28by%20ref%29))
  (bind _charref (Variables|Default|GetCharRef))
  ;[1 1 1] HitDetect
  (if (Actor|ActorHasTag OtherActor "Bullet")
    (Utilities|FlowControl|DoOnce false :!label _label
      (:Completed
        (Variables|Default|SetDamage true)
        (Variables|Default|SetEnemyHealth (- (Variables|Default|GetEnemyHealth) 4e+01))
        (Utilities|FlowControl|Delay 0.1)
        (if (<= (Variables|Default|GetEnemyHealth) 0.0)
          (Variables|/Game/Blueprints/BP_Main.BP_Main_C|SetKills _charref (+ (Variables|/Game/Blueprints/BP_Main.BP_Main_C|GetKills _charref) 1))
          (Actor|DestroyActor)
          (else
            (goto _label Reset)))))))

(event Custom|FollowPlayer
  ;[1 1 1] IA
  (AI|AIMoveTo self "0, 0, 0" (Game|GetPlayerCharacter 0) (Variables|Default|GetAcceptance%20Radius) false
    (:then
      (CallFunction|LookCharacter)
      (Utilities|FlowControl|Delay 2.0)
      (Utilities|FlowControl|DoOnce false :!label _label
        (:Completed
          (Game|SpawnActorfromClass "/Game/Blueprints/BP_BulletEnemy.BP_BulletEnemy_C" (Transformation|GetWorldTransform (Variables|Default|GetPointerEnemy)) "Undefined" "MultiplyWithRoot" 0 0)
          (Utilities|FlowControl|Delay 2.0)
          (goto _label Reset))))))

(event Custom|LifeRegen
  ;[1 1 1] LifeRegeneration
  (if (Variables|Default|GetDamage)
    (Utilities|FlowControl|Delay 1.5)
    (Variables|Default|SetDamage false)
    (else
      (Variables|Default|SetEnemyHealth (+ (Variables|Default|GetEnemyHealth) 0.1))
      (if (>= (Variables|Default|GetEnemyHealth) 1e+02)
        (Variables|Default|SetEnemyHealth 1e+02)))))

(event Custom|Death
  ;[1 1 1] Death
  (if (<= (Variables|Default|GetEnemyHealth) 0.9)
    (Actor|DestroyActor)))

(event EventBeginPlay
  (bind _returnvalue (Actor|GetActorOfClass "/Game/Blueprints/BP_Main.BP_Main_C"))
  (Variables|Default|SetCharRef _returnvalue))

(event EventTick
  (params (DeltaSeconds :type Float%20%28single-precision%29))
  (CallFunction|SetLifeBar)
  (CallFunction|LifeRegen)
  (CallFunction|Death))

(fn ConstructionScript)

(fn LookCharacter
  (bind _returnvalue (Game|GetPlayerCharacter 0))
  (bind _returnvalue_2 (Transformation|GetActorRotation))
  (bind _capsulecomponent (Variables|Collision|GetCapsuleComponent))
  (Utilities|IsValid _returnvalue
    (:Is%20Valid
      (Utilities|IsValid _capsulecomponent
        (:Is%20Valid
          (Transformation|SetWorldRotation _capsulecomponent (Math|Rotator|MakeRotator (.roll _returnvalue_2) (.pitch _returnvalue_2) (.yaw (Math|Rotator|FindLookatRotation (Transformation|GetActorLocation) (Transformation|GetActorLocation _returnvalue)))) false false))))))

(fn SetLifeBar
  (bind _widget (Variables|Default|GetWidget))
  (Utilities|IsValid _widget
    (:Is%20Valid
      (bind _aswb_enemy_health (Utilities|Casting|CastToWB_EnemyHealth (UserInterface|GetWidget _widget)))
      (Progress|SetPercent (Variables|/Game/UI/WB_EnemyHealth.WB_EnemyHealth_C|GetEnemyHealth _aswb_enemy_health) (/ (Variables|Default|GetEnemyHealth) 1e+02)))))