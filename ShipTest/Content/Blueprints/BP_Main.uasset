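; Player pawn for an auto-advancing shooter: creeps along X unless moved manually, turns Cube toward the cursor and fires bullets from two independently cooled-down pointers.
; Tick drives movement, aiming, health regeneration with a post-damage pause, and Score checks on distance and health that open ThirdPersonMap on win or loss.
; It also creates the HUD and pause widgets and spawns enemies through Tick-driven Delays, with only Spawner1 wired up.
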(event Custom|RestoreHealth
  ;[1 1 1] RestoreHealth
  (if (Variables|Default|GetDamage)
    (Utilities|FlowControl|Delay 2.0)
    (Variables|Default|SetDamage false)
    (else
      (Variables|Default|SetHealth (+ (Variables|Default|GetHealth) 0.1))
      (if (>= (Variables|Default|GetHealth) 1e+02)
        (Variables|Default|SetHealth 1e+02)
        (Variables|Default|SetDamage false)))))

(event Custom|AutoMove
  (bind _capsulecomponent (Variables|Default|GetCapsuleComponent))
  (bind _returnvalue (Transformation|GetWorldLocation _capsulecomponent))
  ;[1 1 1] AutoMove
  (if (not (Variables|Default|GetManualMove))
    (Transformation|SetWorldLocation _capsulecomponent (Math|Vector|MakeVector (+ (.x _returnvalue) 0.5) (.y _returnvalue) (.z _returnvalue)) false false)))

(event Custom|Spawner
  (bind _spawner1 (Variables|Default|GetSpawner1))
  (bind _returnvalue (Transformation|GetWorldTransform _spawner1))
  ;[1 1 1] Spawner
  (Utilities|FlowControl|Sequence
    (:then_0
      (Utilities|FlowControl|Delay 4.0)
      (Game|SpawnActorfromClass "/Game/Blueprints/BP_Enemy.BP_Enemy_C" (Math|Transform|MakeTransform (.location _returnvalue) (Math|Rotator|MakeRotator (+ (.roll (.rotation _returnvalue)) 1.8e+02) (.pitch (.rotation _returnvalue)) (.yaw (.rotation _returnvalue))) (.scale _returnvalue)) "Undefined" "MultiplyWithRoot" 0 0))
    (:then_1
      (Utilities|FlowControl|Delay 8.0))
    (:then_2
      (Utilities|FlowControl|Delay 12.0))))

(event Custom|Lose
  ;[1 1 1] Loses
  (bind _returnvalue (Class|Score|CheckLoseCondition (Variables|Default|GetScore) (Math|Float|Truncate (Variables|Default|GetHealth))))
  (if _returnvalue
    (Game|OpenLevel(byName) "ThirdPersonMap")))

(event Custom|WIn
  ;[1 1 1] Wins
  (bind _returnvalue (Class|Score|CheckWinCondition (Variables|Default|GetScore) (Math|Float|Truncate (Variables|Default|GetDistance))))
  (if _returnvalue
    (Game|OpenLevel(byName) "ThirdPersonMap")))

(event Input|EnhancedActionEvents|EnhancedInputActionIA_Move
  (params (ActionValue :type Vector%202D%20Structure) (ElapsedSeconds :type Float%20%28double-precision%29) (TriggeredSeconds :type Float%20%28double-precision%29) (InputAction :type Input%20Action%20Object%20Reference :default "/Game/ThirdPerson/Input/Actions/IA_Move.IA_Move"))
  ;[1 1 1] Movement control
  (:Started
    (Variables|Default|SetManualMove true))
  (:Completed
    (Variables|Default|SetManualMove false)))

(event Input|EnhancedActionEvents|EnhancedInputActionIA_Shoot
  (params (ActionValue :type Vector%202D%20Structure) (ElapsedSeconds :type Float%20%28double-precision%29) (TriggeredSeconds :type Float%20%28double-precision%29) (InputAction :type Input%20Action%20Object%20Reference :default "/Game/ThirdPerson/Input/Actions/IA_Shoot.IA_Shoot"))
  ;[1 1 1] Shoot
  (:Started
    (Utilities|FlowControl|DoOnce false :!label _label
      (:Completed
        (Variables|Default|SetMissileCD true)
        (Game|SpawnActorfromClass "/Game/Blueprints/BP_Bullet.BP_Bullet_C" (Transformation|GetWorldTransform (Variables|Default|GetPointer)) "Undefined" "MultiplyWithRoot" 0 0)
        (Utilities|FlowControl|Delay 2.0)
        (Variables|Default|SetMissileCD false)
        (goto _label Reset)))))

(event Input|EnhancedActionEvents|EnhancedInputActionIA_Shoot2
  (params (ActionValue :type Vector%202D%20Structure) (ElapsedSeconds :type Float%20%28double-precision%29) (TriggeredSeconds :type Float%20%28double-precision%29) (InputAction :type Input%20Action%20Object%20Reference :default "/Game/ThirdPerson/Input/Actions/IA_Shoot2.IA_Shoot2"))
  ;[1 1 1] SecondShoot
  (:Started
    (Utilities|FlowControl|DoOnce false :!label _label
      (:Completed
        (Variables|Default|SetMissileCD2 true)
        (Game|SpawnActorfromClass "/Game/Blueprints/BP_Bullet.BP_Bullet_C" (Transformation|GetWorldTransform (Variables|Default|GetPointer2)) "Undefined" "MultiplyWithRoot" 0 0)
        (Utilities|FlowControl|Delay 2.0)
        (Variables|Default|SetMissileCD2 false)
        (goto _label Reset)))))

(event EventBeginPlay
  (bind _spawner1 (Variables|Default|GetSpawner1))
  (bind _returnvalue (Transformation|GetWorldTransform _spawner1))
  ;[1 1 1] BeginPlay
  (Variables|/Script/Engine.PlayerController|SetbShowMouseCursor (Game|GetPlayerController 0) true)
  (bind _asmy_game_instance (Utilities|Casting|CastToMyGameInstance (Game|GetGameInstance)))
  (Variables|Default|SetGI _asmy_game_instance)
  (bind _returnvalue_2 (UserInterface|CreateWidget "/Game/UI/WB_Interface.WB_Interface_C"))
  (bind _output_get (Variables|Default|SetInterface _returnvalue_2))
  (UserInterface|Viewport|AddtoViewport _output_get 0)
  (bind _returnvalue_3 (UserInterface|CreateWidget "/Game/UI/WB_Pause.WB_Pause_C"))
  (Variables|Default|SetPauseRef _returnvalue_3)
  (Game|SpawnActorfromClass "/Game/Blueprints/BP_Enemy.BP_Enemy_C" (Math|Transform|MakeTransform (.location _returnvalue) (Math|Rotator|MakeRotator (+ (.roll (.rotation _returnvalue)) 1.8e+02) (.pitch (.rotation _returnvalue)) (.yaw (.rotation _returnvalue))) (.scale _returnvalue)) "Undefined" "MultiplyWithRoot" 0 0))

(event EventTick
  (params (DeltaSeconds :type Float%20%28single-precision%29))
  ;[1 1 1] Tick
  (CallFunction|Spawner)
  (CallFunction|LookCursor)
  (CallFunction|RestoreHealth)
  (Variables|Default|SetDistance (Math|Conversions|ToFloat(Integer) (Class|KismetMathLibrary|ToInt64(Float) (.x (Transformation|GetWorldLocation (Variables|Default|GetCapsuleComponent))))))
  (CallFunction|AutoMove)
  (CallFunction|Win)
  (CallFunction|Lose))

(event Input|KeyboardEvents|S
  (params (Key :type Key%20Structure :default "None"))
  ;[1 1 1] Movement control
  (:Pressed
    (Variables|Default|SetManualMove true))
  (:Released
    (Variables|Default|SetManualMove false)))

(event Input|KeyboardEvents|A
  (params (Key :type Key%20Structure :default "None"))
  ;[1 1 1] Movement control
  (:Pressed
    (Variables|Default|SetManualMove false :!label _label))
  (:Released
    (goto _label)))

(event Input|KeyboardEvents|D
  (params (Key :type Key%20Structure :default "None"))
  ;[1 1 1] Movement control
  (:Pressed
    (Variables|Default|SetManualMove false :!label _label))
  (:Released
    (goto _label)))

(event Input|KeyboardEvents|P
  (params (Key :type Key%20Structure :default "None"))
  ;[1 1 1] Pause
  (:Pressed
    (Game|SetGamePaused true)
    (UserInterface|Viewport|AddtoViewport (Variables|Default|GetPauseRef) 0)))

(fn ConstructionScript)

(fn LookCursor
  (bind _returnvalue (Transformation|GetActorRotation))
  (bind _cube (Variables|Default|GetCube))
  (Utilities|IsValid _cube
    (:Is%20Valid
      (Transformation|SetWorldRotation _cube (Math|Rotator|MakeRotator (.roll _returnvalue) (.pitch _returnvalue) (.yaw (Math|Rotator|FindLookatRotation (Transformation|GetActorLocation) (.Location (Collision|BreakHitResult (.HitResult (Game|Player|GetHitResultUnderCursorbyChannel (Game|GetPlayerController 0) "TraceTypeQuery1" true))))))) false false))))